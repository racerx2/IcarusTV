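; Deployable TV device that plays a media stream from a URL on its screen.
; Turning on or starting to run swaps in the screen material and opens the stream; turning off or stopping closes it and applies the off material.
; Interacting calls a client event that only creates the controls widget, as the viewport and input setup is disconnected; GetWidgetClass also supplies that widget class.
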(event `self.ReceiveBeginPlay`
  ;[1 1 1] This is for the TV Stream
)

(event `Client_OpenTVMenu`
  ;[1 1 1] This is for the TV UI
  (bind _returnvalue (`|CreateWidget` "/Game/Mods/TV/UMG_TVControls.UMG_TVControls_C" (`GameplayStatics.GetPlayerController` 0))))

(fn `CheckPower`
  (`MediaPlayer.OpenUrl` (`self.MediaPlayerRef `) (`self.StreamURL`)))

(fn `Deployable_Interact`
  (params (Interactor :type "Actor Object Reference"))
  (`parent.Deployable_Interact` null)
  (`self.Client_OpenTVMenu`))

(fn `GetWidgetClass`
  (returns (Widget :type "UserWidget Class Reference"))
  (return "/Game/Mods/TV/UMG_TVControls.UMG_TVControls_C"))

(fn `OnDeviceStartRunning`
  (`parent.OnDeviceStartRunning`)
  (`PrimitiveComponent.SetMaterial` (`self.TV_Screen`) 0 "/Game/Mods/TV/Materials/M_TV_Screen.M_TV_Screen")
  (`MediaPlayer.OpenUrl` (`self.MediaPlayerRef `) (`self.StreamURL`)))

(fn `OnDeviceStopRunning`
  (`parent.OnDeviceStopRunning`)
  (`MediaPlayer.Close` (`self.MediaPlayerRef `))
  (`PrimitiveComponent.SetMaterial` (`self.TV_Screen`) 0 (`self.TV_OffMaterial`)))

(fn `OnDeviceTurnedOff`
  (`parent.OnDeviceTurnedOff`)
  (`MediaPlayer.Close` (`self.MediaPlayerRef `))
  (`PrimitiveComponent.SetMaterial` (`self.TV_Screen`) 0 (`self.TV_OffMaterial`)))

(fn `OnDeviceTurnedOn`
  (`parent.OnDeviceTurnedOn`)
  (`PrimitiveComponent.SetMaterial` (`self.TV_Screen`) 0 "/Game/Mods/TV/Materials/M_TV_Screen.M_TV_Screen")
  (`MediaPlayer.OpenUrl` (`self.MediaPlayerRef `) (`self.StreamURL`)))

(fn `UserConstructionScript`)